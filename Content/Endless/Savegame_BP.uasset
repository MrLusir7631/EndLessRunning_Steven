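; Endless-game save object that stores player records (name, points, life, distance, time) in an array with an obfuscated Time string.
; SaveData uses Coad to pad each Time character with random key characters before storing.
; LoadGame runs DeCoad, which keeps every fourth character, and returns the record matching a given time.
; As written, it decodes only the first entry repeatedly, and DeCoad blanks all fields except Time.
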(fn `Coad`
  (params (NewParam :type "/Game/ThirdPerson/Blueprints/PlayerST Structure"))
  (returns (NewParam1 :type "/Game/ThirdPerson/Blueprints/PlayerST Structure"))
  (bind (_name _point _life _distance _time) (break `/Game/ThirdPerson/Blueprints/PlayerST` NewParam))
  (for _array_element (`KismetStringLibrary.GetCharacterArrayFromString` _time)
    (set `self.FinalString` (`KismetStringLibrary.Concat_StrStr` (`self.FinalString`) _array_element))
    (for _ (range 4)
      (set `self.FinalString` (`KismetStringLibrary.Concat_StrStr` (`self.FinalString`) (`|GetArrayItem` (`self.RandamKey`) (`KismetMathLibrary.RandomIntegerInRange` 0 8))))))
  (return (make `/Game/ThirdPerson/Blueprints/PlayerST` _name _point _life _distance (`self.FinalString`))))

(fn `DeCoad`
  (params (NewParam :type "/Game/ThirdPerson/Blueprints/PlayerST Structure"))
  (returns (NewParam1 :type "/Game/ThirdPerson/Blueprints/PlayerST Structure"))
  (locals (FinalString :type String))
  (bind _count (`self.Count`))
  (for _array_element (`KismetStringLibrary.GetCharacterArrayFromString` (`.Time_12_209FCDE44457BED8E674DEA8F1634165` (break `/Game/ThirdPerson/Blueprints/PlayerST` NewParam)))
    (if (== (`self.Count`) 0)
      (set `local.FinalString` (`KismetStringLibrary.Concat_StrStr` (`self.FinalString`) _array_element)))
    (`/Engine/EditorBlueprintResources/StandardMacros.IncrementInt` _count
      (:`  `
        (if (>= _count 4)
          (set `self.Count` 0)))))
  (return (make `/Game/ThirdPerson/Blueprints/PlayerST` "" 0 0 0 (`local.FinalString`))))

(fn `Load Game`
  (params (`Dimension 1` :type String))
  (returns (`Player ST` :type "/Game/ThirdPerson/Blueprints/PlayerST Structure"))
  (bind _playerst (`self.PlayerST`))
  (bind _decodest (`self.DeCodeST`))
  (for _ _playerst
    (bind _newparam1 (`self.DeCoad` (`|GetArrayItem` _playerst)))
    (`KismetArrayLibrary.Array_Add` _decodest _newparam1))
  (for _array_element _decodest
    (if (`KismetStringLibrary.EqualEqual_StrStr` (`.Time_12_209FCDE44457BED8E674DEA8F1634165` (break `/Game/ThirdPerson/Blueprints/PlayerST` _array_element)) `Dimension 1`)
      (set `self.Get ST` _array_element)))
  (return (`self.Get ST`)))

(fn `Save Data`
  (params (NewParam :type "/Game/ThirdPerson/Blueprints/PlayerST Structure"))
  (bind _newparam1 (`self.Coad` NewParam))
  (`KismetArrayLibrary.Array_Add` (`self.PlayerST`) _newparam1))